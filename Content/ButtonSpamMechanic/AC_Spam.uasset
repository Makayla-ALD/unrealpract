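; Actor component that runs a button-mashing prompt, asking the player to spam a random Z, X or C key a randomized number of times.
; It creates a WB_SpamBar widget for the prompt and progress, counting each matching press toward the target.
; It fails if no press lands within an initial window or when a retriggerable delay after any key release expires.
; Either outcome calls Completed with the result, then removes the widget and component.
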(event Custom|PressKey
  (Variables|Default|SetAmountPressed (Math|Float|Clamp(Float) (+ (Variables|Default|GetAmountPressed) 1.0) 0.0 (Variables|Default|GetNeededAmount)))
  (CallFunction|UpdateProgressBar)
  (if (== (Variables|Default|GetAmountPressed) (Variables|Default|GetNeededAmount))
    (Default|CallCompleted true)
    (CallFunction|Destroy)))

(event Custom|ReleaseKey
  (Utilities|FlowControl|RetriggerableDelay 0.8)
  (CallFunction|OnFailed))

(event Custom|Destroy
  (bind _widgetreference (Variables|Default|GetWidgetReference)
    (:then
      (Widget|RemovefromParent _widgetreference))
    (:else
      _))
  (Components|DestroyComponent))

(event Custom|OnFailed
  (Variables|Default|SetAmountPressed 0.0)
  (CallFunction|UpdateProgressBar)
  (Default|CallCompleted false)
  (CallFunction|Destroy))

(event EventBeginPlay
  (bind _returnvalue (UserInterface|CreateWidget "/Game/ButtonSpamMechanic/WB_SpamBar.WB_SpamBar_C"))
  (Variables|Default|SetWidgetReference _returnvalue)
  (UserInterface|Viewport|AddtoViewport (Variables|Default|GetWidgetReference) 0)
  (Variables|Default|SetNeededAmount (Math|Random|RandomFloatinRange 1e+01 15.0))
  (Variables|Default|SetKeyPressed (Utilities|Select :Index (Math|Random|RandomInteger 3) :Option%200 "Z" :Option%201 "X" :Option%202 "C"))
  (Rendering|Components|TextRender|SetText (Variables|/Game/ButtonSpamMechanic/WB_SpamBar.WB_SpamBar_C|GetSpamText (Variables|Default|GetWidgetReference)) (Utilities|Text|FormatText "Spam {Key}" (Class|KismetInputLibrary|KeyGetDisplayName (Variables|Default|GetKeyPressed) true)))
  (CallFunction|UpdateProgressBar)
  (Utilities|FlowControl|Delay 4.0)
  (Utilities|IsValid self
    (:Is%20Valid
      (if (<= (Variables|Default|GetAmountPressed) 0.0)
        (CallFunction|OnFailed)))))

(event Input|KeyboardEvents|AnyKey
  (params (Key :type Key%20Structure :default "None"))
  (:Pressed
    (if (== Key (Variables|Default|GetKeyPressed))
      (CallFunction|PressKey)))
  (:Released
    (CallFunction|ReleaseKey)))

(fn UpdateProgressBar
  (Progress|SetPercent (Variables|/Game/ButtonSpamMechanic/WB_SpamBar.WB_SpamBar_C|GetSpamBar (Variables|Default|GetWidgetReference)) (/ (Variables|Default|GetAmountPressed) (Variables|Default|GetNeededAmount))))