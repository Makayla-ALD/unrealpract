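; BP_DNPC is a dialogue NPC that shows its lines one at a time through a WB_Dialogue widget.
; Each Talk event increments Talkindex and writes the matching Dialouge array entry to the widget's TalkText, creating the widget for player 0 if none is valid.
; Once the index passes the last line, it removes the widget from its parent; the index is never reset here.
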(event EventTalk
  (Math|Integer|IncrementInt (Variables|Default|Gettalkindex)
    (:%20%20
      (if (< (Variables|Default|Gettalkindex) (Utilities|Array|Length (Variables|Default|Getdialouge)))
        (Variables|Default|GetUI
          (:then
            _)
          (:else
            (bind _returnvalue (UserInterface|CreateWidget "/Game/Dialogue/WB_Dialogue.WB_Dialogue_C" (Game|GetPlayerController 0)))
            (bind _output_get (Variables|Default|SetUI _returnvalue))
            (UserInterface|Viewport|AddtoViewport _output_get 0)))
        (Rendering|Components|TextRender|SetText (Variables|/Game/Dialogue/WB_Dialogue.WB_Dialogue_C|GetTalkText (Variables|Default|GetUI)) (Utilities|Text|ToText(String) (Utilities|Array|Get(acopy) (Variables|Default|Getdialouge) (Variables|Default|Gettalkindex))))
        (else
          (Widget|RemovefromParent (Variables|Default|GetUI)))))))

(fn ConstructionScript)